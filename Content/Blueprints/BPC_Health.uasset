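; Health component that tracks current health against a maximum, starting full on BeginPlay and refillable through ResetHealth.
; DoDamage subtracts a clamped amount, returns whether the owner is dead, and calls OnDeath only when that hit actually lowered health to zero.
; Each hit also raises an IsDamaged flag and restarts a short timer, which Tick counts down to clear the flag.
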(event Custom|ResetHealth
  ;[1 1 1] ResetHealth
  (Variables|Default|SetCurrent_Health (Variables|Default|GetMax_Health)))

(event EventBeginPlay
  (CallFunction|ResetHealth))

(event EventTick
  (params (DeltaSeconds :type Float%20%28single-precision%29))
  (if (Variables|Default|GetIsDamaged)
    (Variables|Default|SetCurrentDamageTime (- (Variables|Default|GetCurrentDamageTime) DeltaSeconds))
    (if (<= (Variables|Default|GetCurrentDamageTime) 0.0)
      (Variables|Default|SetIsDamaged false))))

(fn GetHealthPercentage
  (return (/ (Variables|Default|GetCurrent_Health) (Variables|Default|GetMax_Health))))

(fn IsDead
  (return (== (CallFunction|GetHealthPercentage) 0.0)))

(fn DoDamage
  (params (Amount :type Float%20%28single-precision%29))
  (bind _isdead (CallFunction|IsDead))
  (Variables|Default|SetCurrentDamageTime 3.0)
  (Variables|Default|SetIsDamaged true)
  (LocalVariables|SetoriginalHealth (Variables|Default|GetCurrent_Health))
  (bind _output_get (Variables|Default|SetCurrent_Health (Math|Float|Clamp(Float) (- (Variables|Default|GetCurrent_Health) Amount) 0.0 (Variables|Default|GetMax_Health))))
  (if (and _isdead (> (LocalVariables|GetoriginalHealth) _output_get))
    (Default|CallOnDeath))
  (return _isdead))