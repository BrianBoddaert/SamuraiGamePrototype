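; BP_VIP is an actor that travels in a straight line from its placed position to a final destination and is destroyed on death.
; Tick plays a Timeline that lerps its location, stopping when health differs from a cached value until the health component's damaged flag clears.
; The construction script records the start and moves component W to the destination.
; The game-over flag logic is disconnected, so death only destroys the actor.
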(event OnDeath(BPC_Health)
  ;[1 1 1] Death
  (Actor|DestroyActor))

(event EventBeginPlay
  (Variables|Default|SetPrevAmountOfHealth (Variables|/Game/Blueprints/BPC_Health.BPC_Health_C|GetCurrent_Health (Variables|Default|GetBPC_Health)))
  (Transformation|SetActorLocation (Variables|Default|GetStartPos) false false))

(event EventTick
  (params (DeltaSeconds :type Float%20%28single-precision%29))
  (bind _bpc_health (Variables|Default|GetBPC_Health))
  (if (== (Variables|Default|GetPrevAmountOfHealth) (Variables|/Game/Blueprints/BPC_Health.BPC_Health_C|GetCurrent_Health (Variables|Default|GetBPC_Health)))
    (bind _alpha (Timeline|Timeline Play)
      (:Update
        (Transformation|SetActorLocation (Math|Vector|Lerp(Vector) (Variables|Default|GetStartPos) (Variables|Default|GetFinalDest) _alpha) false false)))
    (else
      (Utilities|FlowControl|Sequence
        (:then_0
          (Timeline|Timeline Stop))
        (:then_1
          (if (not (Variables|/Game/Blueprints/BPC_Health.BPC_Health_C|GetIsDamaged _bpc_health))
            (Variables|Default|SetPrevAmountOfHealth (Variables|/Game/Blueprints/BPC_Health.BPC_Health_C|GetCurrent_Health _bpc_health))))))))

(fn ConstructionScript
  (Variables|Default|SetStartPos (Transformation|GetActorLocation))
  (Transformation|SetWorldLocation (Variables|Default|Getw) (Variables|Default|GetFinalDest) false false))