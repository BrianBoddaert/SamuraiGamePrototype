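; AI controller for a melee enemy that chases either the player character or the VIP and attacks on arrival.
; A looping timer re-runs target selection, picking TopDownCharacter when it is within range of the pawn, otherwise BP_VIP, and issues AI MoveTo.
; Tick accumulates an attack cooldown; a successful move with the cooldown elapsed always damages the VIP's health component, even when the player is the target.
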(event Custom|MoveToPlayer
  (bind _newparam (CallFunction|SelectTarget))
  (AI|AIMoveTo (Pawn|GetControlledPawn) "0, 0, 0" _newparam 5.0 false
    (:OnSuccess
      (if (>= (Variables|Default|GetAttackTime) 2.0)
        (Variables|Default|SetAttackTime 0.0)
        (bind _returnvalue (Actor|GetActorOfClass "/Game/Blueprints/BP_VIP.BP_VIP_C"))
        (Utilities|IsValid _returnvalue
          (:Is%20Valid
            (Default|DoDamage (Variables|/Game/Blueprints/BP_VIP.BP_VIP_C|GetBPC_Health _returnvalue) 1e+01)))))))

(event EventBeginPlay
  (Utilities|Time|SetTimerbyFunctionName 0 "MoveToPlayer" 1.0 true))

(event EventTick
  (params (DeltaSeconds :type Float%20%28single-precision%29))
  (Variables|Default|SetAttackTime (+ DeltaSeconds (Variables|Default|GetAttackTime))))

(fn ConstructionScript)

(fn SelectTarget
  (bind _returnvalue (Pawn|GetControlledPawn))
  (bind _returnvalue_2 (Actor|GetActorOfClass "/Game/TopDownBP/Blueprints/TopDownCharacter.TopDownCharacter_C"))
  (Utilities|IsValid (Variables|/Script/Engine.Character|GetMesh _returnvalue_2)
    (:Is%20Valid
      (Utilities|IsValid _returnvalue
        (:Is%20Valid
          (if (< (Math|Vector|VectorLength (- (.location (Transformation|GetActorTransform _returnvalue)) (Transformation|GetWorldLocation (Variables|/Script/Engine.Character|GetMesh _returnvalue_2)))) 5e+02)
            (bind _returnvalue_3 (Actor|GetActorOfClass "/Game/TopDownBP/Blueprints/TopDownCharacter.TopDownCharacter_C"))
            (return _returnvalue_3)
            (else
              (bind _returnvalue_4 (Actor|GetActorOfClass "/Game/Blueprints/BP_VIP.BP_VIP_C"))
              (return _returnvalue_4))))))))