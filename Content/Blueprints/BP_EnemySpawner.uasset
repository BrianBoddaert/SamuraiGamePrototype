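; Enemy spawner actor that releases a one-time batch of melee enemies when the VIP enters its trigger box.
; Tick looks up the BP_VIP actor and polls for overlap with the box while spawning is allowed.
; On overlap, a loop spawns AI melee enemies at the spawner's location up to the configured amount, then disables further spawning.
; The construction script shifts the box by a configurable offset, separating trigger area from spawn point.
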(event Custom|Spawn
  (AI|SpawnAIFromClass "/Game/Blueprints/BP_MeleeEnemyCharacter.BP_MeleeEnemyCharacter_C" 0 (.location (Transformation|GetActorTransform)) "0, 0, 0" false 0))

(event EventBeginPlay)

(event Collision|EventActorBeginOverlap
  (params (OtherActor :type Actor%20Object%20Reference)))

(event EventTick
  (params (DeltaSeconds :type Float%20%28single-precision%29))
  (if (Variables|Default|GetCanSpawn)
    (bind _returnvalue (Actor|GetActorOfClass "/Game/Blueprints/BP_VIP.BP_VIP_C"))
    (if (Collision|IsOverlappingActor (Variables|Default|GetBox) _returnvalue :!class /Script/Engine.PrimitiveComponent)
      (while (< (Variables|Default|GetCurrentAmount) (Variables|Default|GetAmountOfEnemiesToSpawn)) :!label _label
        (Variables|Default|SetCurrentAmount (+ (Variables|Default|GetCurrentAmount) 1))
        (CallFunction|Spawn)
        (goto _label))
      (Variables|Default|SetCanSpawn false))))

(fn ConstructionScript
  (Transformation|AddLocalOffset (Variables|Default|GetBox) (Variables|Default|GetOffsetCollider) false false))